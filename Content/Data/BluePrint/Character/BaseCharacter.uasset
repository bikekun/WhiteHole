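; Base character Blueprint that ties a health component and an inventory component to an inventory UI and item pickup.
; Pickup box-traces just ahead of the capsule, passes the hit item's parameters to Inventory, then destroys the actor once added.
; Inventory events refresh the toggleable slot widget, and item stat bonuses currently apply only HP.
; Depleted health triggers Death, which only prints a message.
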(event AddedItem(Inventory)
  (bind _pickupitemref (Variables|Default|GetPickupItemRef))
  ;[1 1 1] Событие добавления предмета в инвентарь \ обновляем виджет
  (Default|UpdateInventorySlots (Variables|Default|GetInventarWidget) (Variables|/Game/Data/BluePrint/Inventory/InventoryComponent/Inventory.Inventory_C|GetItems (Variables|Default|GetInventory)))
  (Utilities|IsValid _pickupitemref
    (:Is%20Valid
      (Actor|DestroyActor _pickupitemref))))

(event AddHealghState(Inventory)
  (params (ItemName :type Text) (AddHP :type Float%20%28single-precision%29) (AddMP :type Float%20%28single-precision%29) (ADdPDP :type Float%20%28single-precision%29) (AddHPRecovery :type Float%20%28single-precision%29) (AddMPRecovery :type Float%20%28single-precision%29))
  ;[1 1 1] Событие передачи инфы об увлечении характеристик
  (Development|PrintString (Utilities|String|Append (Utilities|String|ToString(Float) AddHP) (Utilities|String|ToString(Float) AddMP) (Utilities|String|ToString(Float) ADdPDP) (Utilities|String|ToString(Float) AddHPRecovery) (Utilities|String|ToString(Float) AddMPRecovery) (Utilities|String|ToString(Text) ItemName)))
  (Default|Add (Variables|Default|GetHealthPoint) AddHP))

(event UpdateUMG(Inventory)
  ;[1 1 1] Событие обновить инвентарь
  (Default|UpdateInventorySlots (Variables|Default|GetInventarWidget) (Variables|/Game/Data/BluePrint/Inventory/InventoryComponent/Inventory.Inventory_C|GetItems (Variables|Default|GetInventory))))

(event ValueOff(HealthPoint)
  ;[1 0.03349 0] Смерть
  (CallFunction|Death))

(event Custom|PickupItem
  (bind (_start _end _orintation) (|StartEndSizeGraph_2_2))
  ;[0.3192 0.2543 1] Подборка предмета
  (Variables|Default|SetPickupItemRef 0)
  (bind (_outhits _returnvalue) (Class|KismetSystemLibrary|BoxTraceMulti _start _end "30.000000,30.000000,0.000000" _orintation "TraceTypeQuery1" false 0 "None" true))
  (if _returnvalue
    (bind _array_element (Utilities|Array|ForEachLoopwithBreak _outhits :!label _label)
      (:LoopBody
        (Utilities|IsValid (.HitActor (Collision|BreakHitResult _array_element))
          (:Is%20Valid
            (bind _success (Class|PickUpInterface|PickupCall(Message) (.HitActor (Collision|BreakHitResult _array_element))))
            (if _success
              (goto _label Break)))))
      (:Completed
        (bind _output_get (Variables|Default|SetPickupItemRef (.HitActor (Collision|BreakHitResult _array_element))))
        (bind _asbase_item_actor (Utilities|Casting|CastToBaseItemActor _output_get))
        (Default|AddItem (Variables|Default|GetInventory) (Variables|/Game/Data/BluePrint/Inventory/Items/BaseItemACtor.BaseItemActor_C|GetParameters _asbase_item_actor))))))

(event Custom|ShowCloseInventoryWidget
  (bind _inventarwidget (Variables|Default|GetInventarWidget))
  ;[1 0.085 0.085] Показывает и скрывает окно инвентаря
  (if (Variables|Default|GetIsShowInventary?)
    (Variables|Default|SetIsShowInventary? false)
    (Utilities|IsValid _inventarwidget
      (:Is%20Valid
        (Widget|RemovefromParent _inventarwidget)))
    (else
      (Variables|Default|SetIsShowInventary? true)
      (Utilities|IsValid _inventarwidget
        (:Is%20Valid
          _)
        (:Is%20Not%20Valid
          (CallFunction|CreateInventaryWindow)))
      (UserInterface|Viewport|AddtoViewport (Variables|Default|GetInventarWidget) 0))))

(event Custom|CloseInventoryWidget
  ;[1 0.085 0.085] Показывает и скрывает окно инвентаря
  ;;[1 1 1] Закрыть окно инвентаря
  (if (Variables|Default|GetIsShowInventary?)
    (Variables|Default|SetIsShowInventary? false)
    (Widget|RemovefromParent (Variables|Default|GetInventarWidget))))

(event Custom|Death
  ;[1 0.03349 0] Смерть
  (Development|PrintString "Death" true true "(R=1.000000,G=0.000000,B=0.209591,A=1.000000)" 1e+01))

(event Custom|CustomEvent_2
  (params (SlotNumber :type Integer))
  ;[1 0 0.04893] Использование и выкидывание предметов из инвентаря
)

(event EventUseItemforSlot
  (params (SlotNumber :type Integer))
  ;[1 0 0.04893] Использование и выкидывание предметов из инвентаря
  (Default|UseIteminSlot (Variables|Default|GetInventory) SlotNumber))

(event EventBeginPlay
  (Utilities|IsValid (Variables|Default|GetInventarWidget)
    (:Is%20Not%20Valid
      (CallFunction|CreateInventaryWindow))))

(fn ConstructionScript)

(fn CreateInventaryWindow
  (bind (_rowfill _columnfill) (|ColumnFill&RowFill_2_2))
  (bind _returnvalue (UserInterface|CreateWidget "/Game/Data/UI/Inventory/InventoryWidget.InventoryWidget_C" (Game|GetPlayerController 0)))
  (bind _output_get (Variables|Default|SetInventarWidget _returnvalue))
  (Variables|/Game/Data/UI/Inventory/InventoryWidget.InventoryWidget_C|SetLastColumn _output_get _rowfill)
  (Variables|/Game/Data/UI/Inventory/InventoryWidget.InventoryWidget_C|SetLastRow (Variables|Default|GetInventarWidget) _columnfill)
  (Default|CreateInventarWidget (Variables|Default|GetInventarWidget) (Variables|/Game/Data/BluePrint/Inventory/InventoryComponent/Inventory.Inventory_C|GetItems (Variables|Default|GetInventory)))
  (return))