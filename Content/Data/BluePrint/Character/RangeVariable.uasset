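; RangeVariable is a reusable Blueprint holding a numeric value bounded by ValueMin and ValueMax, with a getter for the current value.
; Events add, subtract or set it, either absolutely or as a fraction of ValueMax, with clamping, or jump it to maximum or zero.
; Every change except Full runs CheckValue, which fires the ValueOff dispatcher at zero or below, regardless of ValueMin.
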(event Custom|Add
  (params (add :type Float%20%28single-precision%29))
  ;[1 1 1] Прибавляет значение
  (bind _output_get (Variables|Default|SetValue (Math|Float|Clamp(Float) (+ add (Variables|Default|GetValue)) (Variables|Default|GetValueMin) (Variables|Default|GetValueMax))))
  (CallFunction|CheckValue _output_get))

(event Custom|Minus
  (params (minus :type Float%20%28single-precision%29))
  ;[1 1 1] Вычитает
  (CallFunction|Add (* minus -1.0)))

(event Custom|CheckValue
  (params (Check :type Float%20%28single-precision%29))
  ;[1 1 1] Проверка значение на минимум и вызыв диспатчера если это так
  (if (<= Check 0.0)
    (Default|CallValueOff)))

(event Custom|Full
  ;[1 1 1] Заполняет до максимуама
  (Variables|Default|SetValue (Variables|Default|GetValueMax)))

(event Custom|AddPercent
  (params (Percent :type Float%20%28single-precision%29))
  ;[1 1 1] Прибавляет процент
  (bind _output_get (Variables|Default|SetValue (Math|Float|Clamp(Float) (+ (* Percent (Variables|Default|GetValueMax)) (Variables|Default|GetValue)) (Variables|Default|GetValueMin) (Variables|Default|GetValueMax))))
  (CallFunction|CheckValue _output_get))

(event Custom|MinusPercent
  (params (Percent :type Float%20%28single-precision%29))
  ;[1 1 1] Вычитает процент
  (CallFunction|AddPercent (* Percent -1.0)))

(event Custom|Zero
  ;[1 1 1] Обнуляет
  (bind _output_get (Variables|Default|SetValue 0.0))
  (CallFunction|CheckValue _output_get))

(event Custom|ChangePercent
  (params (Percent :type Float%20%28single-precision%29))
  ;[1 1 1] Присваевает процент
  (bind _output_get (Variables|Default|SetValue (Math|Float|Clamp(Float) (* Percent (Variables|Default|GetValueMax)) (Variables|Default|GetValueMin) (Variables|Default|GetValueMax))))
  (CallFunction|CheckValue _output_get))

(fn Get
  (return (Variables|Default|GetValue)))